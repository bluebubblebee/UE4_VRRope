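; BP_Rope is a pullable rope in the VR playground that spawns a random pickup when pulled.
; BeginPlay fills an array with pickup and Blooper classes.
; OnPull plays a duck quack at the world origin, then spawns a randomly indexed class from that array at the SpawnPoint component's location.
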(event EventOnPull
  (bind _pickupstospawn (Variables|Default|GetPickupsToSpawn))
  ;[0.4526 0.8066 1] Spawn a random pickup
  (Audio|PlaySoundatLocation "/Game/VRPlayground/Sounds/duck_quack.duck_quack" "0, 0, 0" "0, 0, 0" 1.0 1.0 0.0 0 0 0)
  (Game|SpawnActorfromClass (Utilities|Array|Get(acopy) _pickupstospawn (Math|Random|RandomInteger (Utilities|Array|Length _pickupstospawn))) (Math|Transform|MakeTransform (Transformation|GetWorldLocation (Variables|Default|GetSpawnPoint)) "0, 0, 0" "1,1,1") "Undefined" 0 0))

(event EventBeginPlay
  ;[0.4526 0.8066 1] Initialize Pickups to spawn
  (Variables|Default|SetPickupsToSpawn (Utilities|Array|MakeArray "/Game/VRPlayground/Pickups/BP_Pickup1.BP_Pickup1_C" "/Game/VRPlayground/Pickups/BP_Blooper.BP_Blooper_C" "/Game/VRPlayground/Pickups/BP_Pickup3.BP_Pickup3_C" "/Game/VRPlayground/Pickups/BP_BlooperPickup2.BP_BlooperPickup2_C" "/Game/VRPlayground/Pickups/BP_BlooperPickup3.BP_BlooperPickup3_C" "/Game/VRPlayground/Pickups/BP_Pickup2.BP_Pickup2_C")))

(fn ConstructionScript)